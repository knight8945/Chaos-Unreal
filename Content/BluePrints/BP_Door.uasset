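; An interactive swinging door that the third-person character opens and closes with the E key while inside its trigger volume.
; Trigger overlaps enable or disable input and store the character's capsule; E or DoorToggle drives a FlipFlop that plays or reverses a yaw timeline.
; The GetOpenedDirection result sets the swing's sign, though that function's door-versus-capsule X comparison is left unused.
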(event `self.Door Trigger.OnComponentBeginOverlap`
  (params (OverlappedComponent :type "PrimitiveComponent Object Reference") (OtherActor :type "Actor Object Reference") (OtherComp :type "PrimitiveComponent Object Reference") (OtherBodyIndex :type Integer) (bFromSweep :type Boolean) (SweepResult :type "HitResult Structure (by ref)"))
  ;[1 1 1] Door Trigger
  (bind _asbp_third_person_character (cast `/Game/ThirdPerson/Blueprints/BP_ThirdPersonCharacter` OtherActor))
  (`self.EnableInput` (`GameplayStatics.GetPlayerController` 0))
  (set `self.Capsule Component` (`Character.CapsuleComponent` _asbp_third_person_character)))

(event `self.Door Trigger.OnComponentEndOverlap`
  (params (OverlappedComponent :type "PrimitiveComponent Object Reference") (OtherActor :type "Actor Object Reference") (OtherComp :type "PrimitiveComponent Object Reference") (OtherBodyIndex :type Integer))
  ;[1 1 1] Door Trigger
  (cast `/Game/ThirdPerson/Blueprints/BP_ThirdPersonCharacter` OtherActor)
  (`self.DisableInput` (`GameplayStatics.GetPlayerController` 0)))

(event `Door Toggle`
  (bind _door (`self.Door`))
  ;[1 1 1] Door Opening
  (`/Engine/EditorBlueprintResources/StandardMacros.FlipFlop` :!label _label
    (:`A`
      (set `self. isFront` (`self.GetOpenedDirection`))
      (bind (_direction _rotation_z) (`Timeline|DoorOpenTimeline` :!label _label_2)
        (:`Update`
          (if (`self. isFront`)
            (`SceneComponent.K2_SetRelativeRotation` _door (`KismetMathLibrary.MakeRotator` 0.0 0.0 _rotation_z) false false)
            (else
              (`SceneComponent.K2_SetRelativeRotation` _door (`KismetMathLibrary.MakeRotator` 0.0 0.0 (* _rotation_z -1.0)) false false))))))
    (:`B`
      (goto _label_2 :!via `Reverse`))))

(event `Key|E`
  (params (Key :type "Key Structure"))
  ;[1 1 1] Door Opening
  (:`Pressed`
    (goto _label)))

(fn `UserConstructionScript`)