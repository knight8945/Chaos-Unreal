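; BP_Bouncy_Ball is a breakable ball actor that launches itself in a random direction on spawn.
; The construction script randomizes the sphere's scale, and BeginPlay applies a mass-scaled random impulse.
; Its Break event spawns a DestructableObject and an FS_MasterField at the sphere's transform, triggers the field to drive the destruction, then destroys the ball.
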(event `self.ReceiveBeginPlay`
  (`PrimitiveComponent.AddImpulse` (`self.Sphere`) (* (`KismetMathLibrary.RandomUnitVector`) (`KismetMathLibrary.RandomFloatInRange` 1000.0 3000.0) (`PrimitiveComponent.GetMass` (`self.Sphere`))) "None" false))

(event `Break`
  (bind _returnvalue (`SceneComponent.K2_GetComponentToWorld` (`self.Sphere`)))
  (`|SpawnActorFromClass` (`self.DestructableObject`) _returnvalue "Undefined" "MultiplyWithRoot" null null)
  (bind _returnvalue_2 (`|SpawnActorFromClass` "/Engine/EditorResources/FieldNodes/FS_MasterField.FS_MasterField_C" _returnvalue "Undefined" "MultiplyWithRoot" null null))
  (set `/Engine/EditorResources/FieldNodes/FS_MasterField.ActivationType` "NewEnumerator4" _returnvalue_2)
  (`/Engine/EditorResources/FieldNodes/FS_MasterField.CE_Trigger` _returnvalue_2)
  (`self.K2_DestroyActor`))

(fn `UserConstructionScript`
  (`SceneComponent.SetRelativeScale3D` (`self.Sphere`) (`KismetMathLibrary.Conv_DoubleToVector` (`KismetMathLibrary.RandomFloatInRange` 0.2 0.3))))