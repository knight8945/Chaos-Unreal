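; BP_Collectables is a pickup that, when the third-person character overlaps it, adds score through BP_ThirdPersonGameMode and destroys itself.
; On BeginPlay it starts two timelines, one yawing the root component and one bobbing the Sphere vertically around a raised offset.
; Each timeline's Finished pin calls its own event again, so the spin and float repeat for as long as the item exists.
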(event `self.ReceiveActorBeginOverlap`
  (params (OtherActor :type "Actor Object Reference"))
  (cast `/Game/ThirdPerson/Blueprints/BP_ThirdPersonCharacter` OtherActor)
  (bind _asbp_third_person_game_mode (cast `/Game/ThirdPerson/Blueprints/BP_ThirdPersonGameMode` (`GameplayStatics.GetGameMode`)))
  (`/Game/ThirdPerson/Blueprints/BP_ThirdPersonGameMode.AddScore` _asbp_third_person_game_mode)
  (`self.K2_DestroyActor`))

(event `self.ReceiveBeginPlay`
  (`self.RotateMe`)
  (`self.Floating`))

(event `RotateMe`
  (bind (_direction _itemrotatez) (`Timeline|ItemRotateTimeline` :!via `PlayFromStart`)
    (:`Update`
      (`SceneComponent.K2_SetRelativeRotation` (`self.DefaultSceneRoot`) (`KismetMathLibrary.MakeRotator` 0.0 0.0 _itemrotatez) false false))
    (:`Finished`
      (`self.RotateMe`))))

(event `Floating`
  (bind (_direction _itemlocationz) (`Timeline|ItemFloatTimeline` :!via `PlayFromStart`)
    (:`Update`
      (`SceneComponent.K2_SetRelativeLocation` (`self.Sphere`) (`KismetMathLibrary.MakeVector` 0.0 0.0 (+ (* _itemlocationz 20.0) 120.0)) false false))
    (:`Finished`
      (`self.Floating`))))

(fn `UserConstructionScript`)