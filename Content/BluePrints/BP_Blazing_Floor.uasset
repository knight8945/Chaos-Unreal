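; BP_Blazing_Floor is a floor hazard that periodically damages the player standing on it.
; Box overlap events store the overlapping BP_ThirdPersonCharacter as StandingPlayer and clear it when such a character leaves.
; A looping one-second timer started on BeginPlay applies fixed damage to that character while the reference is valid, tracking only one at a time.
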(event `self.Box.OnComponentBeginOverlap`
  (params (OverlappedComponent :type "PrimitiveComponent Object Reference") (OtherActor :type "Actor Object Reference") (OtherComp :type "PrimitiveComponent Object Reference") (OtherBodyIndex :type Integer) (bFromSweep :type Boolean) (SweepResult :type "HitResult Structure (by ref)"))
  (bind _asbp_third_person_character (cast `/Game/ThirdPerson/Blueprints/BP_ThirdPersonCharacter` OtherActor))
  (set `self.Standing Player` _asbp_third_person_character))

(event `self.Box.OnComponentEndOverlap`
  (params (OverlappedComponent :type "PrimitiveComponent Object Reference") (OtherActor :type "Actor Object Reference") (OtherComp :type "PrimitiveComponent Object Reference") (OtherBodyIndex :type Integer))
  (cast `/Game/ThirdPerson/Blueprints/BP_ThirdPersonCharacter` OtherActor)
  (set `self.Standing Player` null))

(event `self.ReceiveBeginPlay`
  (`KismetSystemLibrary.K2_SetTimerDelegate` (delegate `DamagePlayer`) 1.0 true))

(event `DamagePlayer`
  (bind _standing_player (`self.Standing Player`))
  (`/Engine/EditorBlueprintResources/StandardMacros.IsValid` _standing_player
    (:`Is Valid`
      (`GameplayStatics.ApplyDamage` _standing_player 20.0))))

(fn `UserConstructionScript`)